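; Weapon actor that handles ammo and fire-rate gating, with no projectile or damage logic of its own.
; UseWeapon spends one round if ammo remains and the rate lock is clear, then locks use until the UseRate timer calls StopRateDelay.
; With AutoFire, StopRateDelay calls UseWeapon again until StopUseWeapon or a failed attempt clears FireActive.
; Interact sets it as CurrentWeapon on the player's weapon manager; CurrentAmmo's OnRep is empty.
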(event EventBeginPlay)

(event Collision|EventActorBeginOverlap
  (params (OtherActor :type Actor%20Object%20Reference)))

(event EventTick
  (params (DeltaSeconds :type Float%20%28single-precision%29)))

(fn ConstructionScript)

(fn UseWeapon
  (bind _out (CallFunction|AbletoUseWeapon))
  (if _out
    (Math|Integer|DecrementInt (Variables|Default|GetCurrentAmmo)
      (:%20%20
        (Utilities|Time|SetTimerbyFunctionName 0 "StopRateDelay" (Variables|Default|GetUseRate))
        (Variables|Default|SetUseFreezedByRate true)
        (if (Variables|Default|GetAutoFire)
          (Variables|Default|SetFireActive true))
        (return true)))
    (else
      (Variables|Default|SetFireActive false)
      (return false))))

(fn AbletoUseWeapon
  (return (and (> (Variables|Default|GetCurrentAmmo) 0) (not (Variables|Default|GetUseFreezedByRate)))))

(fn StopRateDelay
  (Variables|Default|SetUseFreezedByRate false)
  (if (and (Variables|Default|GetAutoFire) (Variables|Default|GetFireActive))
    (CallFunction|UseWeapon)))

(fn StopUseWeapon
  (Variables|Default|SetFireActive false))

(fn OnRepCurrentAmmo)

(fn Interact
  (params (PlayerCharacter :type BP%20Player%20Character%20Object%20Reference))
  (Variables|/Game/Blueprints/Components/Player/BP_WeaponManager.BP_WeaponManager_C|SetCurrentWeapon (Variables|/Game/Blueprints/Player/BP_PlayerCharacter.BP_PlayerCharacter_C|GetBP_WeaponManager PlayerCharacter) self)
  (return false))