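; Player health component that tracks health, armor and death for BP_PlayerCharacter.
; On the server it binds to the owner's damage event, scales damage down by current armor, then drains health and depletes armor at twice the reduced damage.
; Health at zero or below sets Dead, whose RepNotify calls CallCharDead and disables character movement, with debug messages for damage and death.
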(event Custom|OnPlayerTakeAnyDamage
  (params (DamagedActor :type Actor%20Object%20Reference) (Damage :type Float%20%28single-precision%29) (DamageType :type Damage%20Type%20Object%20Reference) (InstigatedBy :type Controller%20Object%20Reference) (DamageCauser :type Actor%20Object%20Reference))
  (CallFunction|ApplyDamage Damage))

(event EventBeginPlay
  (bind _asbp_player_character (Utilities|Casting|CastToBP_PlayerCharacter (Components|GetOwner)))
  (bind _output_get (Variables|Default|SetCharacter _asbp_player_character))
  (if (Networking|IsServer)
    (EventDispatchers|AssignOnTakeAnyDamage _output_get (delegate Custom|OnPlayerTakeAnyDamage))))

(event EventTick
  (params (DeltaSeconds :type Float%20%28single-precision%29)))

(fn ApplyDamage
  (params (Damage :type Float%20%28single-precision%29))
  (bind _output_get (LocalVariables|SetL_Damage (* Damage (- 1.0 (/ (Variables|Default|GetArmor) 2e+02)))))
  (CallFunction|PringMessage (Utilities|String|Append "Damage: " (Utilities|String|ToString(Float) _output_get)) "(R=0.846497,G=1.000000,B=0.064000,A=1.000000)" 2.0 false)
  (Variables|Default|SetHealth (- (Variables|Default|GetHealth) (LocalVariables|GetL_Damage)))
  (Variables|Default|SetArmor (Math|Float|Max(Float) (- (Variables|Default|GetArmor) (* (LocalVariables|GetL_Damage) 2.0)) 0.0))
  (if (<= (Variables|Default|GetHealth) 0.0)
    (Variables|Default|SetDead true)))

(fn OnRepDead
  (if (Variables|Default|GetDead)
    (Default|CallCharDead)
    (Pawn|Components|CharacterMovement|DisableMovement (Variables|/Script/Engine.Character|GetCharacterMovement (Variables|Default|GetCharacter)))
    (if (Networking|IsServer)
      (CallFunction|PringMessage "CHAR DEAD!!!!" "(R=0.928000,G=0.000000,B=0.000000,A=1.000000)" 3.0 false))))