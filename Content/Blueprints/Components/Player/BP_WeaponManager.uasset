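; Player character component that manages the weapon inventory: main, secondary, melee, and lists of specials and grenades.
; CreateWeapon spawns a weapon, files it by type and attaches it to the character.
; Selection sets CurrentWeapon by type; scrolling cycles only main, secondary and melee.
; OnRep_CurrentWeapon attaches it to the visible mesh's weapon socket on clients, returning the previous one to the character, while the server attaches it to the character.
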(event Custom|SelectWeaponFromClient
  (params (Type :type E_WeaponType%20Enum :default "NewEnumerator0"))
  (CallFunction|SelectWeapon Type))

(event Custom|ScrollWeaponFromClient
  (params (Next :type Boolean))
  (CallFunction|ScrollWeapon Next))

(event EventBeginPlay
  (bind _asbp_player_character (Utilities|Casting|CastToBP_PlayerCharacter (Components|GetOwner)))
  (Variables|Default|SetCharacter _asbp_player_character))

(event EventTick
  (params (DeltaSeconds :type Float%20%28single-precision%29)))

(fn CreateWeapon
  (params (Class :type BP%20Weapon%20Class%20Reference))
  (bind _character (Variables|Default|GetCharacter))
  (bind _returnvalue (Game|SpawnActorfromClass Class (Math|Transform|MakeTransform "0, 0, 0" "0, 0, 0" "1,1,1") "AlwaysSpawn" (Pawn|GetController _character) _character))
  (bind _output_get (LocalVariables|SetL_Weapon _returnvalue))
  (switch Utilities|FlowControl|Switch|SwitchonE_WeaponType (Variables|/Game/Blueprints/Weapons/BP_Weapon.BP_Weapon_C|GetWeaponType _output_get)
    (:NewEnumerator0
      (Variables|Default|SetMainWeapon (LocalVariables|GetL_Weapon)))
    (:NewEnumerator1
      (Variables|Default|SetSecondWeapon (LocalVariables|GetL_Weapon)))
    (:NewEnumerator2
      (Utilities|Array|Add (Variables|Default|GetSpecialWeapon) (LocalVariables|GetL_Weapon)))
    (:NewEnumerator3
      (Utilities|Array|Add (Variables|Default|GetGrenades) (LocalVariables|GetL_Weapon)))
    (:NewEnumerator4
      (Variables|Default|SetMeleeWeapon (.AsBP%20Melee%20Weapon (Utilities|Casting|CastToBP_MeleeWeapon (LocalVariables|GetL_Weapon))))))
  (Transformation|AttachActorToActor (LocalVariables|GetL_Weapon) (Variables|Default|GetCharacter) "None" "SnapToTarget" "SnapToTarget" "KeepRelative" true)
  (return (LocalVariables|GetL_Weapon) 0))

(fn OnRepCurrentWeapon
  (if (not (Networking|IsServer))
    (bind _clientweaponattached (Variables|Default|GetClientWeaponAttached)
      (:then
        (Transformation|AttachActorToActor _clientweaponattached (Variables|Default|GetCharacter) " None" "SnapToTarget" "SnapToTarget" "KeepRelative" true))
      (:else
        _))
    (Transformation|AttachComponentToComponent (Variables|Default|GetCurrentWeapon) (Default|GetVisibleMesh (Variables|Default|GetCharacter)) "SKT_Weapon" "KeepRelative" "KeepRelative" "KeepRelative" true)
    (Variables|Default|SetClientWeaponAttached (Variables|Default|GetCurrentWeapon))
    (CallFunction|PringMessage "Weapon attached" "(R=0.000000,G=0.033985,B=0.944000,A=1.000000)" 2.0 false)
    (else
      (Transformation|AttachActorToActor (Variables|Default|GetCurrentWeapon) (Variables|Default|GetCharacter) "None" "SnapToTarget" "SnapToTarget" "KeepRelative" true))))

(fn SelectWeapon
  (params (Type :type E_WeaponType%20Enum :default "NewEnumerator0") (Index :type Integer))
  (bind _mainweapon (Variables|Default|GetMainWeapon))
  (bind _secondweapon (Variables|Default|GetSecondWeapon))
  (bind _specialweapon (Variables|Default|GetSpecialWeapon))
  (bind _grenades (Variables|Default|GetGrenades))
  (bind _meleeweapon (Variables|Default|GetMeleeWeapon))
  (bind _output (Utilities|Array|Get(acopy) _specialweapon Index))
  (bind _output_2 (Utilities|Array|Get(acopy) _grenades Index))
  (bind _returnvalue (Utilities|Select :Index Type :NewEnumerator0 _mainweapon :NewEnumerator1 _secondweapon :NewEnumerator2 _output :NewEnumerator3 _output_2 :NewEnumerator4 _meleeweapon))
  (Utilities|IsValid _returnvalue
    (:Is%20Valid
      (bind _output_get (Variables|Default|SetCurrentWeapon _returnvalue))
      (return _output_get))
    (:Is%20Not%20Valid
      (return (Variables|Default|GetCurrentWeapon)))))

(fn ScrollWeapon
  (params (Next :type Boolean))
  (bind _currentweapon (Variables|Default|GetCurrentWeapon)
    (:then
      (if Next
        (switch Utilities|FlowControl|Switch|SwitchonE_WeaponType (Variables|/Game/Blueprints/Weapons/BP_Weapon.BP_Weapon_C|GetWeaponType _currentweapon)
          (:NewEnumerator0
            (CallFunction|SelectWeaponfromClient "NewEnumerator1"))
          (:NewEnumerator1
            (CallFunction|SelectWeaponfromClient "NewEnumerator4"))
          (:NewEnumerator4
            (CallFunction|SelectWeaponfromClient "NewEnumerator0")))
        (else
          (switch Utilities|FlowControl|Switch|SwitchonE_WeaponType (Variables|/Game/Blueprints/Weapons/BP_Weapon.BP_Weapon_C|GetWeaponType _currentweapon)
            (:NewEnumerator0
              (CallFunction|SelectWeaponfromClient "NewEnumerator4"))
            (:NewEnumerator1
              (CallFunction|SelectWeaponfromClient "NewEnumerator0"))
            (:NewEnumerator4
              (CallFunction|SelectWeaponfromClient "NewEnumerator1"))))))
    (:else)))