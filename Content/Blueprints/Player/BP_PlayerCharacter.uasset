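; First-person, networked player character handling movement, look, jump, weapon use and interaction.
; Fire, reload and interact inputs call server events that drive the current weapon or message the actor hit by a short camera line trace.
; BPWeaponManager handles scroll and number-key switching, and on possession the authority creates rifle, pistol and knife, equipping the rifle.
; GetVisibleMesh returns the hands mesh for the local player, otherwise the body mesh.
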(event Custom|Server_Fire
  (params (Activate :type Boolean))
  ;[1 1 1] Fire from weapon
  (bind _currentweapon (Variables|/Game/Blueprints/Components/Player/BP_WeaponManager.BP_WeaponManager_C|GetCurrentWeapon (Variables|Default|GetBP_WeaponManager))
    (:then
      (if Activate
        (Default|UseWeapon _currentweapon)
        (else
          (Default|StopUseWeapon _currentweapon))))
    (:else)))

(event Custom|ServerReloadWeapon
  (bind _currentweapon (Variables|/Game/Blueprints/Components/Player/BP_WeaponManager.BP_WeaponManager_C|GetCurrentWeapon (Variables|Default|GetBP_WeaponManager))
    (:then
      (bind _asbp_fire_weapons (Utilities|Casting|CastToBP_FireWeapons _currentweapon))
      (Variables|/Game/Blueprints/Weapons/BP_FireWeapons.BP_FireWeapons_C|SetReloading _asbp_fire_weapons true))
    (:else)))

(event Custom|ServerInteract
  (bind (_hit _hitresult) (CallFunction|InteractTrace))
  (if _hit
    (Class|BPInteractionInterface|Interact(Message) (.HitActor (Collision|BreakHitResult _hitresult)) self)))

(event EventPossessed
  (params (NewController :type Controller%20Object%20Reference))
  (Networking|SwitchHasAuthority
    (:Authority
      (bind _weapon (Default|CreateWeapon (Variables|Default|GetBP_WeaponManager) "/Game/Blueprints/Weapons/BP_Weapon_AutoRifles.BP_Weapon_AutoRifles_C"))
      (Variables|/Game/Blueprints/Components/Player/BP_WeaponManager.BP_WeaponManager_C|SetCurrentWeapon (Variables|Default|GetBP_WeaponManager) _weapon)
      (Default|CreateWeapon (Variables|Default|GetBP_WeaponManager) "/Game/Blueprints/Weapons/BP_Weapon_Pistol.BP_Weapon_Pistol_C")
      (Default|CreateWeapon (Variables|Default|GetBP_WeaponManager) "/Game/Blueprints/Weapons/BP_Weapon_Knife.BP_Weapon_Knife_C"))))

(event Collision|EventActorBeginOverlap
  (params (OtherActor :type Actor%20Object%20Reference)))

(event EventTick
  (params (DeltaSeconds :type Float%20%28single-precision%29)))

(event Input|ActionEvents|InputActionFire
  (params (Key :type Key%20Structure))
  ;[1 1 1] Fire from weapon
  (:Pressed
    (CallFunction|ServerFire true))
  (:Released
    (CallFunction|ServerFire false)))

(event Input|ActionEvents|InputActionInteract
  (params (Key :type Key%20Structure))
  (bind (_hit _hitresult) (CallFunction|InteractTrace))
  (:Pressed
    (if _hit
      (if (Utilities|DoesObjectImplementInterface (.HitActor (Collision|BreakHitResult _hitresult)) "/Game/Blueprints/Libs/Interfaces/BP_InteractionInterface.BP_InteractionInterface_C")
        (CallFunction|ServerInteract)))))

(event Input|ActionEvents|InputActionJump
  (params (Key :type Key%20Structure))
  (:Pressed
    (Character|Jump)))

(event Input|ActionEvents|InputActionReload
  (params (Key :type Key%20Structure))
  (:Pressed
    (bind _currentweapon (Variables|/Game/Blueprints/Components/Player/BP_WeaponManager.BP_WeaponManager_C|GetCurrentWeapon (Variables|Default|GetBP_WeaponManager))
      (:then
        (Utilities|Casting|CastToBP_FireWeapons _currentweapon)
        (CallFunction|ServerReloadWeapon))
      (:else))))

(event Input|AxisEvents|InputAxisLookUp
  (params (AxisValue :type Float%20%28single-precision%29))
  (Pawn|Input|AddControllerPitchInput AxisValue))

(event Input|AxisEvents|InputAxisTurn
  (params (AxisValue :type Float%20%28single-precision%29))
  (Pawn|Input|AddControllerYawInput AxisValue))

(event Input|AxisEvents|InputAxisMoveForward
  (params (AxisValue :type Float%20%28single-precision%29))
  (Pawn|Input|AddMovementInput (Transformation|GetActorForwardVector) AxisValue false))

(event Input|AxisEvents|InputAxisMoveRight
  (params (AxisValue :type Float%20%28single-precision%29))
  (Pawn|Input|AddMovementInput (Transformation|GetActorRightVector) AxisValue false))

(event Input|KeyboardEvents|1
  (params (Key :type Key%20Structure))
  (:Pressed
    (Default|SelectWeaponfromClient (Variables|Default|GetBP_WeaponManager) "NewEnumerator0")))

(event Input|KeyboardEvents|2
  (params (Key :type Key%20Structure))
  (:Pressed
    (Default|SelectWeaponfromClient (Variables|Default|GetBP_WeaponManager) "NewEnumerator1")))

(event Input|MouseEvents|MouseWheelDown
  (params (Key :type Key%20Structure))
  (:Pressed
    (Default|ScrollWeaponfromClient (Variables|Default|GetBP_WeaponManager) false)))

(event Input|MouseEvents|MouseWheelUp
  (params (Key :type Key%20Structure))
  (:Pressed
    (Default|ScrollWeaponfromClient (Variables|Default|GetBP_WeaponManager) true)))

(event Input|KeyboardEvents|3
  (params (Key :type Key%20Structure))
  (:Pressed
    (Default|SelectWeaponfromClient (Variables|Default|GetBP_WeaponManager) "NewEnumerator4")))

(fn ConstructionScript)

(fn GetVisibleMesh
  (return (select (Pawn|IsLocallyControlled) (Variables|Default|GetHandsMesh) (Variables|Character|GetMesh))))

(fn InteractTrace
  (bind _camera (Variables|Default|GetCamera))
  (bind _returnvalue (Transformation|GetWorldLocation _camera))
  (bind (_outhit _returnvalue_2) (Collision|LineTraceByChannel _returnvalue (+ _returnvalue (* (Transformation|GetActorForwardVector (Pawn|GetController)) 5e+02)) "TraceTypeQuery1" false 0 "None"))
  (return _returnvalue_2 _outhit))